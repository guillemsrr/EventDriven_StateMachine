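; BP_RoomManager is a level actor that shows a room and repositions the orbital camera pivot as its collision volume is entered.
; Any begin overlap reveals the root and its children, then passes CameraPivot to the ArcherPlayerCameraManager.
; End overlap hides them again only for an ArcherCharacter; the matching cast for begin overlap is disconnected.
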(event OnComponentBeginOverlap(PlayerCollision)
  (params (OverlappedComponent :type Primitive%20Component%20Object%20Reference) (OtherActor :type Actor%20Object%20Reference) (OtherComp :type Primitive%20Component%20Object%20Reference) (OtherBodyIndex :type Integer) (bFromSweep :type Boolean) (SweepResult :type Hit%20Result%20Structure%20%28by%20ref%29))
  (Rendering|SetVisibility (Variables|Default|GetRoot) true true)
  (bind _asarcher_player_camera_manager (Utilities|Casting|CastToArcherPlayerCameraManager (Game|GetPlayerCameraManager 0)))
  (Class|ArcherPlayerCameraManager|SetOrbitalCameraPivotPoint _asarcher_player_camera_manager (Variables|Default|GetCameraPivot)))

(event OnComponentEndOverlap(PlayerCollision)
  (params (OverlappedComponent :type Primitive%20Component%20Object%20Reference) (OtherActor :type Actor%20Object%20Reference) (OtherComp :type Primitive%20Component%20Object%20Reference) (OtherBodyIndex :type Integer))
  (Utilities|Casting|CastToArcherCharacter OtherActor)
  (Rendering|SetVisibility (Variables|Default|GetRoot) false true))

(fn ConstructionScript)